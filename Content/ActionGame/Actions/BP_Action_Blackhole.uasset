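; BP_Action_Blackhole is the Blackhole ability action, gated by and paid for with the instigator's Rage attribute.
; CanStart requires both the parent check to pass and Rage to be at least RageCost.
; StartAction runs the parent logic, deducts RageCost through the attributes component, then immediately stops the action, leaving any blackhole behavior to the parent class.
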(event `self.StartAction`
  (params (Instigator :type "Actor Object Reference"))
  (`parent.StartAction` Instigator)
  (bind _returnvalue (`SAttributeComponent.GetAttributes` Instigator))
  (`SAttributeComponent.ApplyRageChange` _returnvalue (* (`self.RageCost`) -1.0))
  (`self.StopAction` Instigator))

(fn `CanStart`
  (params (Instigator :type "Actor Object Reference"))
  (returns (ReturnValue :type Boolean))
  (bind _returnvalue (`parent.CanStart` Instigator))
  (bind _returnvalue_2 (`SAttributeComponent.GetAttributes` Instigator))
  (return (and _returnvalue (>= (`SAttributeComponent.Rage` _returnvalue_2) (`self.RageCost`)))))