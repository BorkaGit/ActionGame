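; Custom EQS generator that produces candidate cover points around the querier.
; It casts visibility traces every 10 degrees from a ring at Radius inward to the querier's navmesh-projected location.
; Each hit is pushed out along its surface normal, placing the point on the side of the obstacle facing away from the querier.
; Points are gathered in a set, then added as query items.
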(fn `DoItemGeneration`
  (params (ContextLocations :type "Array of Vector Structure (by ref)"))
  (`KismetArrayLibrary.Array_Clear` (`self.LocationSet`))
  (for _index (range 36)
    (bind _asactor (cast `Actor` (`self.GetQuerier`)))
    (bind _projectedlocation (`NavigationSystemV1.K2_ProjectPointToNavigation` (`Actor.K2_GetActorLocation` _asactor) null "/Script/NavigationSystem.RecastFilter_UseDefaultArea"))
    (bind (_outhit _returnvalue) (`KismetSystemLibrary.LineTraceSingle` :`Start` (+ (* (`KismetMathLibrary.GreaterGreater_VectorRotator` (1.0 0.0 0.0) (`KismetMathLibrary.MakeRotator` 0.0 0.0 (* _index 10.0))) (`self.Radius`)) _projectedlocation) :`End` _projectedlocation :`TraceChannel` "TraceTypeQuery1" :`DrawDebugType` "ForOneFrame"))
    (if _returnvalue
      (bind (_bblockinghit _binitialoverlap _time _distance _location _impactpoint _normal _impactnormal) (`GameplayStatics.BreakHitResult` _outhit))
      (`KismetArrayLibrary.Array_Add` (`self.LocationSet`) (+ _impactpoint (* _impactnormal 50)))))
  (for _array_element (`self.LocationSet`)
    (`self.AddGeneratedVector` _array_element))
  (return))