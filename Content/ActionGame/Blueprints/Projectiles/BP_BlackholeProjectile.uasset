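; Black hole projectile that swallows physics-simulating objects it overlaps.
; On BeginPlay its sphere collider ignores the instigator while moving, and hits on any other actor spawn an emitter at the projectile's location.
; Sphere overlaps destroy the other actor if the overlapped component simulates physics.
; A RadialForce component is present but not driven by the graph, which also never destroys the projectile itself.
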(event `self.ReceiveBeginPlay`
  (`PrimitiveComponent.IgnoreActorWhenMoving` (`self.SphereComp`) (`self.GetInstigator`) true))

(event `self.SphereComp.OnComponentHit`
  (params (HitComponent :type "PrimitiveComponent Object Reference") (OtherActor :type "Actor Object Reference") (OtherComp :type "PrimitiveComponent Object Reference") (NormalImpulse :type "Vector Structure") (Hit :type "HitResult Structure (by ref)"))
  (if (!= OtherActor (`self.GetInstigator`))
    (`GameplayStatics.SpawnEmitterAtLocation` null (`self.K2_GetActorLocation`))))

(event `self.SphereComp.OnComponentBeginOverlap`
  (params (OverlappedComponent :type "PrimitiveComponent Object Reference") (OtherActor :type "Actor Object Reference") (OtherComp :type "PrimitiveComponent Object Reference") (OtherBodyIndex :type Integer) (bFromSweep :type Boolean) (SweepResult :type "HitResult Structure (by ref)"))
  (if (`SceneComponent.IsSimulatingPhysics` OtherComp "None")
    (`self.K2_DestroyActor` OtherActor)))

(fn `UserConstructionScript`)