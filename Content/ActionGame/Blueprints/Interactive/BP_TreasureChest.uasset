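; BP_TreasureChest is an interactive chest that a pawn can open and close if it holds the required key card.
; Interact checks the pawn's SActionComponent active gameplay tags for an exact RequiredKeyCard match.
; A FlipFlop alternates playing and reversing the AnimateLid timeline, which drives the lid mesh's pitch.
; The timeline's Finished output activates the particle system.
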(event `SGameplayInterface.Interact`
  (params (InstigatorPawn :type "Pawn Object Reference"))
  (if (`BlueprintGameplayTagLibrary.HasTag` (`SActionComponent.ActiveGameplayTags` (`self.GetComponentByClass` InstigatorPawn "/Script/ActionGame.SActionComponent")) (`self.RequiredKeyCard`) true)
    (`/Engine/EditorBlueprintResources/StandardMacros.FlipFlop`
      (:`A`
        (bind (_direction _pitch) (`Timeline|AnimateLid` :!label _label)
          (:`Update`
            (`SceneComponent.K2_SetRelativeRotation` (`self.LidMesh`) (`KismetMathLibrary.MakeRotator` 0.0 _pitch) false false))
          (:`Finished`
            (`ActorComponent.Activate` (`self.ParticleSystem`) false))))
      (:`B`
        (goto _label :!via `Reverse`)))))

(fn `UserConstructionScript`)